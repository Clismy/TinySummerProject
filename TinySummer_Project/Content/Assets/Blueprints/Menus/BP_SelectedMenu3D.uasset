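; Actor that displays the selected submenu (Settings, How to Play, Scoreboard or Credits) as a 3D widget in the menus.
; SelectedMenu hides the cached TempWidget, switches it to the chosen widget component, then makes it visible and enables its user widget.
; Deactivate disables input on the current user widget through SetIsEnabled but leaves the component visible.
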(event `self.ReceiveBeginPlay`)

(event `SelectedMenu`
  (params (selectedMenu :type "/Game/Assets/Widgets/SelectedMenuEnums Enum" :default "NewEnumerator0"))
  (bind _tempwidget (`self.TempWidget`))
  (`/Engine/EditorBlueprintResources/StandardMacros.IsValid` (`self.TempWidget`)
    (:`Is Valid`
      (`SceneComponent.SetVisibility` (`self.TempWidget`) false false))
    (:`Is Not Valid`
      _))
  (switch `/Game/Assets/Widgets/SelectedMenuEnums` selectedMenu
    (:`NewEnumerator0`
      (set `self.TempWidget` (`self.Settings_Widget`)))
    (:`NewEnumerator1`
      (set `self.TempWidget` (`self.HowToPlay_Widget`)))
    (:`NewEnumerator2`
      (set `self.TempWidget` (`self.Scoreboard_Widget`)))
    (:`NewEnumerator3`
      (set `self.TempWidget` (`self.Credits_Widget`))))
  (`SceneComponent.SetVisibility` _tempwidget true false)
  (`Widget.SetIsEnabled` (`WidgetComponent.GetUserWidgetObject` _tempwidget) true))

(event `Deactivate`
  (bind _tempwidget (`self.TempWidget`))
  (`/Engine/EditorBlueprintResources/StandardMacros.IsValid` _tempwidget
    (:`Is Valid`
      (`Widget.SetIsEnabled` (`WidgetComponent.GetUserWidgetObject` _tempwidget) false))))

(fn `UserConstructionScript`)