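; GameTimer is a manager actor that runs a 30-second countdown and keeps the current score.
; It creates WBP_HUD on BeginPlay and writes the time and score into its text variables.
; Tick counts down while enabled; at zero it waits briefly, tells LevelManager to switch to the menu, then stops.
; SetPlayTimer toggles the countdown, resetting time and score when stopped, while AddTime and AddScore increase them.
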(event `self.ReceiveBeginPlay`
  ;[1 1 1] cc
  (bind _returnvalue (`|CreateWidget` "/Game/Assets/Widgets/WBP_HUD.WBP_HUD_C" (`GameplayStatics.GetPlayerController` 0)))
  (bind _output_get (set `self.As WBP HUD` _returnvalue))
  (`UserWidget.AddToViewport` _output_get 0)
  (set `self.Timer` 30.0))

(event `self.ReceiveTick`
  (params (DeltaSeconds :type "Float (single-precision)"))
  ;[1 1 1] cc
  (if (`self.ShouldPlayTimer`)
    (set `self.Timer` (- (`self.Timer`) DeltaSeconds))
    (set `/Game/Assets/Widgets/WBP_HUD.MyText` (`KismetStringLibrary.Conv_DoubleToString` (`self.Timer`)) (`self.As WBP HUD`))
    (if (<= (`self.Timer`) 0.0)
      (set `self.Timer` 0.0)
      (set `/Game/Assets/Widgets/WBP_HUD.MyText` (`KismetStringLibrary.Conv_DoubleToString` (`self.Timer`)) (`self.As WBP HUD`))
      (`KismetSystemLibrary.Delay` 0.5)
      (bind _returnvalue (`GameplayStatics.GetActorOfClass` "/Game/Assets/Blueprints/Managers/LevelManager.LevelManager_C"))
      (`/Game/Assets/Blueprints/Managers/LevelManager.SwitchToMenu` _returnvalue)
      (`self.SetPlayTimer` false))))

(event `SetPlayTimer`
  (params (ShouldPlayTimer :type Boolean))
  ;[1 1 1] cc
  (if (not ShouldPlayTimer)
    (set `self.Timer` 30.0)
    (set `self.Highscore` 0))
  (set `self.ShouldPlayTimer` ShouldPlayTimer))

(event `AddScore`
  (params (Score :type Integer))
  ;[1 1 1] cc
  (bind _output_get (set `self.Highscore` (+ Score (`self.Highscore`))))
  (set `/Game/Assets/Widgets/WBP_HUD.myHighscore` (`KismetStringLibrary.Conv_IntToString` _output_get) (`self.As WBP HUD`)))

(event `AddTime`
  (params (Score :type "Float (double-precision)"))
  ;[1 1 1] cc
  (set `self.Timer` (+ Score (`self.Timer`))))

(fn `UserConstructionScript`)