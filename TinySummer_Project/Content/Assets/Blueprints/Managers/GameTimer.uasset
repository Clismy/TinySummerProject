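; GameTimer is a manager actor that runs the match countdown and tracks the player's score.
; While active, Tick uses a one-second Delay to decrement Seconds, then stops the timer and calls ResetMatch on LevelManager at zero.
; AddSeconds (capped at a minute) and AddScore trigger HUD feedback.
; Each active tick also checks score milestones, telling EnemySpawner to update its settings when one is reached.
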(event `self.ReceiveTick`
  (params (DeltaSeconds :type "Float (single-precision)"))
  ;[1 1 1] Update
  (if (`self.ShouldPlayTimer`)
    (`self.UpdateScoreMilestone`)
    (`KismetSystemLibrary.Delay` 1.0)
    (if (== (`self.Seconds`) 0)
      (`self.SetPlayTimer` false)
      (bind _returnvalue (`GameplayStatics.GetActorOfClass` "/Game/Assets/Blueprints/Managers/LevelManager.LevelManager_C"))
      (`/Game/Assets/Blueprints/Managers/LevelManager.ResetMatch` _returnvalue)
      (else
        (set `self.Seconds` (- (`self.Seconds`) 1))))))

(event `AddSeconds`
  (params (Seconds :type Integer))
  (bind _returnvalue (+ Seconds (`self.Seconds`)))
  ;[1 1 1] AddSeconds
  (set `self.TimeAdded` Seconds)
  (if (> _returnvalue 60)
    (set `self.TempSeconds` (- _returnvalue 60))
    (set `self.Seconds` 60)
    (else
      (set `self.Seconds` _returnvalue)))
  (`/Game/Assets/Widgets/WBP_HUD.PlayTimePopup` (`self.As WBP HUD`)))

(event `SetPlayTimer`
  (params (ShouldPlayTimer :type Boolean))
  ;[1 1 1] SetPlayTimer
  (if ShouldPlayTimer
    (set `self.Seconds` (`self.StartSeconds`))
    (else
      (set `self.Highscore` 0)))
  (set `self.ShouldPlayTimer` ShouldPlayTimer))

(event `AddScore`
  (params (Score :type Integer))
  (bind _as_wbp_hud (`self.As WBP HUD`))
  ;[1 1 1] AddScore
  (set `self.ScoreAdded` Score)
  (set `self.Highscore` (+ Score (`self.Highscore`)))
  (`/Game/Assets/Widgets/WBP_HUD.PlayScorePopup` _as_wbp_hud)
  (`/Game/Assets/Widgets/WBP_HUD.CrosshairHit` _as_wbp_hud))

(fn `UpdateScoreMilestone`
  (if (>= (`self.Highscore`) (`self.nextMileStone`))
    (set `self.nextMileStone` (+ (`self.nextMileStone`) (`self.mileStoneAmount`)))
    (bind _returnvalue (`GameplayStatics.GetActorOfClass` "/Game/Assets/Blueprints/Managers/EnemySpawner.EnemySpawner_C"))
    (`/Game/Assets/Blueprints/Managers/EnemySpawner.UpdateSettings` _returnvalue)))

(fn `UserConstructionScript`)