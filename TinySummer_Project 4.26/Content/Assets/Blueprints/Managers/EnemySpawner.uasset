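; Enemy spawner manager that periodically places Cardboard_new enemies at SpawnPoint actors in the level.
; On BeginPlay it gathers all spawn points, then a looping timer spawns at a random listed point while ShouldPlay is set, capped at six live enemies.
; Each enemy receives its point and a spawner reference, and that point leaves the list until AddPoint puts one back.
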(event `Spawner`
  (bind _randint (`self.RandInt`))
  (bind _spawnpointlist (`self.spawnPointList`))
  (bind _output (`|GetArrayItem` _spawnpointlist _randint))
  ;[1 1 1] Comment
  (if (`self.ShouldPlay`)
    (set `self.RandInt` (`KismetMathLibrary.RandomInteger` (- (`KismetArrayLibrary.Array_Length` _spawnpointlist) 1)))
    (bind _outactors (`GameplayStatics.GetAllActorsOfClass` "/Game/Assets/Blueprints/Enemy/Cardboard_new.Cardboard_new_C"))
    (if (<= (`KismetArrayLibrary.Array_Length` (`self.spawnPointList`)) 0)
      _
      (elif (< (`KismetArrayLibrary.Array_Length` _outactors) 6)
        (bind _returnvalue (`|SpawnActorFromClass` "/Game/Assets/Blueprints/Enemy/Cardboard_new.Cardboard_new_C" (`self.GetTransform` _output) "Undefined" "OverrideRootScale" null null))
        (`/Game/Assets/Blueprints/Enemy/Cardboard_new.SetSpawnPoint` _returnvalue _output)
        (`/Game/Assets/Blueprints/Enemy/Cardboard_new.SetEnemySpawner` _returnvalue self)
        (`KismetArrayLibrary.Array_Remove` (`self.spawnPointList`) _randint)))))

(event `self.ReceiveBeginPlay`
  ;[1 1 1] Comment
  (bind _outactors (`GameplayStatics.GetAllActorsOfClass` "/Game/Assets/Blueprints/Enemy/SpawnPoint.SpawnPoint_C"))
  (set `self.spawnPointList` _outactors)
  (`KismetSystemLibrary.K2_SetTimerDelegate` (delegate `Spawner`) 3.0 true))

(event `AddPoint`
  (params (spawnPoint :type "/Game/Assets/Blueprints/Enemy/SpawnPoint Object Reference"))
  ;[1 1 1] Comment
  (`KismetArrayLibrary.Array_Add` (`self.spawnPointList`) spawnPoint))

(event `SetShouldPlay`
  (params (ShouldPlay :type Boolean))
  ;[1 1 1] Comment
  (set `self.ShouldPlay` ShouldPlay))

(fn `UserConstructionScript`)