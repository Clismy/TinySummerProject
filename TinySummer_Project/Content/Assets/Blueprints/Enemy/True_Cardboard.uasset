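; Pop-up cardboard shooting target that appears as either an enemy or a civilian, chosen by a weighted random roll.
; Tick despawns it when its lifetime runs out, wiggling shortly before; each activation shortens that lifetime, and Milestone raises the civilian odds.
; Hit scores head or body by component name, feeds combo, score and time to GameTimer, then returns the target to EnemySpawner after the despawn animation.
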(event `Reset`
  ;[1 1 1] Reset
  (`self.Hit` null)
  (set `self.CivWeight` 0.0))

(event `Hit`
  (params (HitCompontent :type "ActorComponent Object Reference") (GotHit :type Boolean))
  ;[1 1 1] Hit
  (if (not (`self.IsDead`))
    (`self.CalculatePoints` HitCompontent)
    (`|ExecutionSequence`
      (:`then_0`
        (`self.PlayCardboardDeSpawn`)
        (set `self.DeathTimer` 0.0)
        (bind _returnvalue (`AnimSequenceBase.GetPlayLength` (select `int` 0 :`0` "/Game/Assets/Animations/Enemies/ANIM_enemyPopcorn_despawn.ANIM_enemyPopcorn_despawn" :`1` null :`2` null :!type "AnimSequenceBase Object Reference")))
        (`KismetSystemLibrary.Delay` _returnvalue)
        (`/Game/Assets/Blueprints/Managers/EnemySpawner.AddCardboard` (`self.Enemy Spawner`) self)
        (set `self.calledCount` 0)
        (`self.ResetCardboard`)
        (set `self.IsDead` true))
      (:`then_1`
        (if GotHit
          (bind _returnvalue_2 (`GameplayStatics.GetActorOfClass` "/Game/Assets/Blueprints/Managers/GameTimer.GameTimer_C"))
          (`/Game/Assets/Blueprints/Managers/GameTimer.AddCombo` _returnvalue_2 (`self.CardboardEnum`))
          (`/Game/Assets/Blueprints/Managers/GameTimer.AddScore` _returnvalue_2 (`self.ScoreToAdd`))
          (if (`self.ShouldAddTime`)
            (`/Game/Assets/Blueprints/Managers/GameTimer.AddSeconds` _returnvalue_2 (`self.TimeToAdd`))
            (`self.PlayHeadSound`)
            (else
              (`self.PlayBodySound`))))))))

(event `self.ReceiveBeginPlay`
  ;[1 1 1] Event Begin
  (bind _returnvalue (`GameplayStatics.GetActorOfClass` "/Game/Assets/Blueprints/Managers/EnemySpawner.EnemySpawner_C"))
  (set `self.Enemy Spawner` _returnvalue)
  (`SceneComponent.SetVisibility` (`self.Civ`) false false)
  (`SceneComponent.SetVisibility` (`self.Enemy`) false false))

(event `Activate`
  ;[1 1 1] Activate Cardboard
  (`self.DetermineCardboardType`)
  (`self.SetCardboard`)
  (`self.PlayCardboardSpawn`)
  (set `self.DeathRate` (`KismetMathLibrary.FClamp` (* (`self.DeathRate`) 0.96) 1.0 10.0))
  (set `self.IsDead` false))

(event `self.ReceiveTick`
  (params (DeltaSeconds :type "Float (single-precision)"))
  ;[1 1 1] Update
  (if (`self.IsDead`)
    _
    (elif (>= (`self.DeathTimer`) (`self.DeathRate`))
      (`self.Hit` null)
      (else
        (set `self.DeathTimer` (+ (`self.DeathTimer`) DeltaSeconds))
        (if (>= (`self.DeathTimer`) (* (`self.DeathRate`) 0.8))
          (if (not (`SkeletalMeshComponent.IsPlaying` (`self.SkeletalMesh`)))
            (`self.PlayCardboardWiggle`)))))))

(event `Milestone`
  ;[1 1 1] Milestone
  (set `self.CivWeight` (`KismetMathLibrary.FClamp` (+ (`self.CivWeight`) 0.009) 0.0 0.2)))

(fn `CalculatePoints`
  (params (HitCompontent :type "ActorComponent Object Reference"))
  (bind _returnvalue (`KismetSystemLibrary.GetObjectName` HitCompontent))
  (`/Engine/EditorBlueprintResources/StandardMacros.IsValid` HitCompontent
    (:`Is Valid`
      (if (`KismetStringLibrary.EqualEqual_StrStr` (`KismetSystemLibrary.GetObjectName` (`self.Head`)) _returnvalue)
        (`self.SetHeadScore`)
        (elif (`KismetStringLibrary.EqualEqual_StrStr` (`KismetSystemLibrary.GetObjectName` (`self.Body`)) _returnvalue)
          (`self.SetBodyScore`)))
      (return))
    (:`Is Not Valid`
      (return))))

(fn `DetermineCardboardType`
  (if (`KismetMathLibrary.RandomBoolWithWeight` (`self.CivWeight`))
    (set `self.CardboardEnum` "NewEnumerator1")
    (else
      (set `self.CardboardEnum` "NewEnumerator0"))))

(fn `PlayBodySound`
  (`GameplayStatics.GetActorOfClass` "/Game/Assets/Blueprints/Managers/LevelManager.LevelManager_C")
  (switch `/Game/Assets/Blueprints/Enemy/CardboardEnum` (`self.CardboardEnum`)
    (:`NewEnumerator0`
      (`GameplayStatics.PlaySound2D` "/Game/Assets/Audio/SFX/Enemy/SFX_bodyshot_Cue.SFX_bodyshot_Cue" 1.0 1.0 0.0 null null))
    (:`NewEnumerator1`
      (`GameplayStatics.PlaySound2D` "/Game/Assets/Audio/SFX/Enemy/SFX_civillianHit_Cue.SFX_civillianHit_Cue" 1.0 1.0 0.0 null null))))

(fn `PlayCardboardDeSpawn`
  (`SkeletalMeshComponent.PlayAnimation` (`self.SkeletalMesh`) "/Game/Assets/Animations/Enemies/ANIM_enemyPopcorn_despawn.ANIM_enemyPopcorn_despawn" false))

(fn `PlayCardboardSpawn`
  (`SkeletalMeshComponent.PlayAnimation` (`self.SkeletalMesh`) "/Game/Assets/Animations/Enemies/ANIM_enemyPopcorn_spawn.ANIM_enemyPopcorn_spawn" false))

(fn `PlayCardboardWiggle`
  (`SkeletalMeshComponent.PlayAnimation` (`self.SkeletalMesh`) "/Game/Assets/Animations/Enemies/ANIM_enemyPopcorn_wiggle.ANIM_enemyPopcorn_wiggle" false))

(fn `PlayHeadSound`
  (`GameplayStatics.GetActorOfClass` "/Game/Assets/Blueprints/Managers/LevelManager.LevelManager_C")
  (switch `/Game/Assets/Blueprints/Enemy/CardboardEnum` (`self.CardboardEnum`)
    (:`NewEnumerator0`
      (`GameplayStatics.PlaySound2D` "/Game/Assets/Audio/SFX/Enemy/SFX_headshot_Cue.SFX_headshot_Cue" 1.0 1.0 0.0 null null))
    (:`NewEnumerator1`
      (`GameplayStatics.PlaySound2D` "/Game/Assets/Audio/SFX/Enemy/SFX_civillianHit_Cue.SFX_civillianHit_Cue" 1.0 1.0 0.0 null null))))

(fn `ResetCardboard`
  (switch `/Game/Assets/Blueprints/Enemy/CardboardEnum` (`self.CardboardEnum`)
    (:`NewEnumerator0`
      (`SceneComponent.SetVisibility` (`self.Enemy`) false false))
    (:`NewEnumerator1`
      (`SceneComponent.SetVisibility` (`self.Civ`) false false))))

(fn `SetBodyScore`
  (switch `/Game/Assets/Blueprints/Enemy/CardboardEnum` (`self.CardboardEnum`)
    (:`NewEnumerator0`
      (set `self.ScoreToAdd` (`self.EnemyBodyScore`))
      (set `self.TimeToAdd` 0)
      (set `self.ShouldAddTime` false))
    (:`NewEnumerator1`
      (set `self.ScoreToAdd` (`self.CivBodyScore`))
      (set `self.TimeToAdd` (`self.CivBodyTime`))
      (set `self.ShouldAddTime` true)))
  (return))

(fn `SetCardboard`
  (switch `/Game/Assets/Blueprints/Enemy/CardboardEnum` (`self.CardboardEnum`)
    (:`NewEnumerator0`
      (`SceneComponent.SetVisibility` (`self.Enemy`) true false))
    (:`NewEnumerator1`
      (`SceneComponent.SetVisibility` (`self.Civ`) true false))))

(fn `SetHeadScore`
  (switch `/Game/Assets/Blueprints/Enemy/CardboardEnum` (`self.CardboardEnum`)
    (:`NewEnumerator0`
      (set `self.ScoreToAdd` (`self.EnemyHeadScore`))
      (set `self.TimeToAdd` (`self.EnemyHeadTime`))
      (set `self.ShouldAddTime` true))
    (:`NewEnumerator1`
      (set `self.ScoreToAdd` (`self.CivHeadScore`))
      (set `self.TimeToAdd` (`self.CivHeadTime`))
      (set `self.ShouldAddTime` true)))
  (return))

(fn `UserConstructionScript`)