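; Pop-up cardboard enemy target that awards score when hit and hides itself if left standing too long.
; Hit scores by struck component name (Head, Body, Feet), updating GameTimer with points, plus bonus seconds for headshots, and playing matching sounds.
; Tick triggers a non-scoring Hit once DeathRate elapses; after the despawn animation, it reports back to EnemySpawner.
; Each Activate respawns it with a 5% shorter, unclamped lifetime.
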(event `Hit`
  (params (HitCompontent :type "ActorComponent Object Reference") (GotHit :type Boolean))
  ;[1 1 1] Hit
  (if (not (`self.IsDead`))
    (set `self.IsDead` true)
    (`self.CalculatePoints` HitCompontent)
    (`|ExecutionSequence`
      (:`then_0`
        (`SkeletalMeshComponent.PlayAnimation` (`self.SkeletalMesh`) "/Game/Assets/Animations/Enemies/ANIM_enemyPopcorn_despawn.ANIM_enemyPopcorn_despawn" false)
        (set `self.DeathTimer` 0.0)
        (bind _returnvalue (`AnimSequenceBase.GetPlayLength` (select `int` 0 :`0` "/Game/Assets/Animations/Enemies/ANIM_enemyPopcorn_despawn.ANIM_enemyPopcorn_despawn" :`1` null :`2` null :!type "AnimSequenceBase Object Reference")))
        (`KismetSystemLibrary.Delay` _returnvalue)
        (`/Game/Assets/Blueprints/Managers/EnemySpawner.AddNewPoints` (`self.Enemy Spawner`) self)
        (set `self.calledCount` 0))
      (:`then_1`
        (if GotHit
          (bind _returnvalue_2 (`GameplayStatics.GetActorOfClass` "/Game/Assets/Blueprints/Managers/GameTimer.GameTimer_C"))
          (`/Game/Assets/Blueprints/Managers/GameTimer.AddScore` _returnvalue_2 (`self.ScoreToAdd`))
          (if (`self.ShouldAddTime`)
            (`/Game/Assets/Blueprints/Managers/GameTimer.AddSeconds` _returnvalue_2 (`self.TotalSeconds`))
            (`KismetSystemLibrary.Delay` 0.1)
            (`GameplayStatics.PlaySound2D` "/Game/Assets/Audio/SFX/Enemy/SFX_headshot_Cue.SFX_headshot_Cue" 1.0 1.0 0.0 null null)
            (else
              (`KismetSystemLibrary.Delay` 0.1)
              (`GameplayStatics.PlaySound2D` "/Game/Assets/Audio/SFX/Enemy/SFX_bodyshot_Cue.SFX_bodyshot_Cue" 1.0 1.0 0.0 null null))))))))

(event `self.ReceiveBeginPlay`
  ;[1 1 1] Event Begin
  (bind _returnvalue (`GameplayStatics.GetActorOfClass` "/Game/Assets/Blueprints/Managers/EnemySpawner.EnemySpawner_C"))
  (set `self.Enemy Spawner` _returnvalue))

(event `Activate`
  ;[1 1 1] Activate Cardboard
  (if (`self.IsDead`)
    (set `self.DeathRate` (* (`self.DeathRate`) 0.95))
    (`SkeletalMeshComponent.PlayAnimation` (`self.SkeletalMesh`) "/Game/Assets/Animations/Enemies/ANIM_enemyPopcorn_spawn.ANIM_enemyPopcorn_spawn" false)
    (set `self.IsDead` false)))

(event `self.ReceiveTick`
  (params (DeltaSeconds :type "Float (single-precision)"))
  ;[1 1 1] Update
  (if (`self.IsDead`)
    _
    (elif (>= (`self.DeathTimer`) (`self.DeathRate`))
      (`self.Hit` null)
      (else
        (set `self.DeathTimer` (+ (`self.DeathTimer`) DeltaSeconds))))))

(fn `CalculatePoints`
  (params (`Hit Compontent` :type "ActorComponent Object Reference"))
  (`/Engine/EditorBlueprintResources/StandardMacros.IsValid` `Hit Compontent`
    (:`Is Valid`
      (switch `string` (`KismetSystemLibrary.GetObjectName` `Hit Compontent`)
        (:`Head`
          (set `self.ShouldAddTime` true)
          (set `self.ScoreToAdd` (`self.HeadScore`)))
        (:`Body`
          (set `self.ShouldAddTime` false)
          (set `self.ScoreToAdd` (`self.BodyScore`)))
        (:`Feet`
          (set `self.ShouldAddTime` false)
          (set `self.ScoreToAdd` (`self.FeetScore`))))
      (return))
    (:`Is Not Valid`
      (return))))

(fn `UserConstructionScript`)