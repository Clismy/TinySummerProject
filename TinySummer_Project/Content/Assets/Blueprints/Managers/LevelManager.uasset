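; Level manager that moves the game between the 3D main menu, first-person play and the result screen.
; Switch events play camera sequences for menu transitions and toggle HUD, cursor and player control.
; Entering play starts the GameTimer, EnemySpawner and music, and lets F end the turn early once.
; Results fire confetti, while ResetMatch stops spawning and music, resets cardboard targets and plays game-over sounds.
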(event `self.ReceiveBeginPlay`
  ;[1 1 1] Begin Play
  (bind _returnvalue (`|CreateWidget` "/Game/Assets/Widgets/WBP_HUD.WBP_HUD_C" (`GameplayStatics.GetPlayerController` 0)))
  (bind _output_get (set `self.HUDWidgetRef` _returnvalue))
  (`Widget.SetVisibility` _output_get "Hidden")
  (`UserWidget.AddToViewport` _output_get 0)
  (bind _asfirst_person_character (cast `/Game/Assets/Blueprints/Player/FirstPersonCharacter` (`GameplayStatics.GetPlayerCharacter` 0)))
  (set `self.FirstPersonRef` _asfirst_person_character)
  (bind _returnvalue_2 (`GameplayStatics.GetActorOfClass` "/Game/Assets/Blueprints/Managers/GameTimer.GameTimer_C"))
  (set `self.GameTimerRef` _returnvalue_2))

(event `InputAction|F`
  (params (Key :type "Key Structure"))
  ;[1 1 1] EndTurn
  (:`Pressed`
    (if (`self.CanSkip`)
      (`/Game/Assets/Blueprints/Managers/GameTimer.EarlyEnd` (`self.GameTimerRef`))
      (set `self.CanSkip` false))))

(event `SwitchToMenu`
  ;[1 1 1] Switch Player To Menu
  (set `self.IsGameFinished` false)
  (set `PlayerController.bShowMouseCursor` false (`GameplayStatics.GetPlayerController` 0))
  (`/Game/Assets/Blueprints/Player/FirstPersonCharacter.DisablePlayer` (`self.FirstPersonRef`) false)
  (`Widget.SetVisibility` (`self.HUDWidgetRef`) "Hidden")
  (bind _returnvalue (`GameplayStatics.GetActorOfClass` "/Game/Assets/Blueprints/Menus/MenuCamera.MenuCamera_C"))
  (`PlayerController.SetViewTargetWithBlend` (`GameplayStatics.GetPlayerController` 0) _returnvalue 0.0 "VTBlend_Linear" 0.0 false)
  (bind _returnvalue_2 (`GameplayStatics.GetActorOfClass` "/Game/Assets/Blueprints/Managers/LevelSequenceManager.LevelSequenceManager_C"))
  (`/Game/Assets/Blueprints/Managers/LevelSequenceManager.PlaySequence` _returnvalue_2 (`self.CameraToMenu`) false)
  (bind _timelength (`/Game/Assets/Blueprints/Managers/LevelSequenceManager.TimeLength` _returnvalue_2))
  (`KismetSystemLibrary.Delay` _timelength)
  (set `PlayerController.bShowMouseCursor` true (`GameplayStatics.GetPlayerController` 0))
  (bind _returnvalue_3 (`GameplayStatics.GetActorOfClass` "/Game/Assets/Blueprints/Menus/BP_MainMenu3D.BP_MainMenu3D_C"))
  (`/Game/Assets/Blueprints/Menus/BP_MainMenu3D.EnableMenu` _returnvalue_3))

(event `ToPlayer`
  ;[1 1 1] To Player
  (`/Game/Assets/Blueprints/Player/FirstPersonCharacter.ActivatePlayer` (`self.FirstPersonRef`))
  (bind _returnvalue (`GameplayStatics.GetActorOfClass` "/Game/Assets/Blueprints/Managers/GameTimer.GameTimer_C"))
  (`/Game/Assets/Blueprints/Managers/GameTimer.SetPlayTimer` _returnvalue true)
  (bind _returnvalue_2 (`GameplayStatics.GetActorOfClass` "/Game/Assets/Blueprints/Managers/EnemySpawner.EnemySpawner_C"))
  (`/Game/Assets/Blueprints/Managers/EnemySpawner.SetShouldPlay` _returnvalue_2 true)
  (`Widget.SetVisibility` (`self.HUDWidgetRef`) "Visible"))

(event `SwitchResultToPlayer`
  ;[1 1 1] Switch Result To Player
  (set `PlayerController.bShowMouseCursor` false (`GameplayStatics.GetPlayerController` 0))
  (set `self.IsGameFinished` false)
  (`Widget.SetVisibility` (`self.HUDWidgetRef`) "Visible")
  (`SceneComponent.SetVisibility` (`/Game/Assets/Blueprints/Player/FirstPersonCharacter.PlayerHands` (`self.FirstPersonRef`)) true false)
  (`self.ToPlayer`)
  (bind _returnvalue (`GameplayStatics.SpawnSound2D` "/Game/Assets/Audio/Music/BGM_level0_Cue.BGM_level0_Cue" 1.0 1.0 0.0 null))
  (set `self.BGM_Level` _returnvalue)
  (`KismetSystemLibrary.Delay` 0.2)
  (set `self.CanSkip` true))

(event `SwitchMenuToPlayer`
  ;[1 1 1] Switch Menu To Player
  (set `PlayerController.bShowMouseCursor` false (`GameplayStatics.GetPlayerController` 0))
  (bind _returnvalue (`GameplayStatics.GetActorOfClass` "/Game/Assets/Blueprints/Managers/LevelSequenceManager.LevelSequenceManager_C"))
  (`/Game/Assets/Blueprints/Managers/LevelSequenceManager.PlaySequence` _returnvalue (`self.CameraToPlayer`) false)
  (`SceneComponent.SetVisibility` (`/Game/Assets/Blueprints/Player/FirstPersonCharacter.PlayerHands` (`self.FirstPersonRef`)) true false)
  (`KismetSystemLibrary.Delay` (`TimeManagementBlueprintLibrary.Conv_QualifiedFrameTimeToSeconds` (`MovieSceneSequencePlayer.GetDuration` (`/Game/Assets/Blueprints/Managers/LevelSequenceManager.SequencePlayer` _returnvalue))))
  (`PlayerController.SetViewTargetWithBlend` (`GameplayStatics.GetPlayerController` 0) (`self.FirstPersonRef`) 0.0 "VTBlend_Linear" 0.0 false)
  (`self.ToPlayer`)
  (bind _returnvalue_2 (`GameplayStatics.SpawnSound2D` "/Game/Assets/Audio/Music/BGM_level0_Cue.BGM_level0_Cue" 1.0 1.0 0.0 null))
  (set `self.BGM_Level` _returnvalue_2)
  (`KismetSystemLibrary.Delay` 0.2)
  (set `self.CanSkip` true))

(event `SwitchPlayerToResult`
  (bind _confettilocation (`self.ConfettiLocation`))
  (bind _confettilocation2 (`self.ConfettiLocation2`))
  ;[1 1 1] Switch Player To Result
  (`Widget.SetVisibility` (`self.HUDWidgetRef`) "Hidden")
  (`/Game/Assets/Blueprints/Player/FirstPersonCharacter.DisablePlayer` (`self.FirstPersonRef`) false)
  (`GameplayStatics.SpawnEmitterAtLocation` "/Game/Assets/Animations/VFX/Confetti/P_confetti.P_confetti" _confettilocation (`self.ConfettiRotation`))
  (`GameplayStatics.PlaySoundAtLocation` "/Game/Assets/Audio/SFX/Environment/SFX_confetti_cue.SFX_confetti_cue" _confettilocation (struct) 1.0 1.0 0.0 null null null)
  (`KismetSystemLibrary.Delay` 0.1)
  (`GameplayStatics.SpawnEmitterAtLocation` "/Game/Assets/Animations/VFX/Confetti/P_confetti.P_confetti" _confettilocation2 (`self.ConfettiRotation2`))
  (`GameplayStatics.PlaySoundAtLocation` "/Game/Assets/Audio/SFX/Environment/SFX_confetti_cue.SFX_confetti_cue" _confettilocation2 (struct) 1.0 1.0 0.0 null null null)
  (set `self.IsGameFinished` true)
  (set `PlayerController.bShowMouseCursor` true (`GameplayStatics.GetPlayerController` 0)))

(event `ResetMatch`
  ;[1 1 1] ResetMatch
  (bind _returnvalue (`GameplayStatics.GetActorOfClass` "/Game/Assets/Blueprints/Managers/EnemySpawner.EnemySpawner_C"))
  (`/Game/Assets/Blueprints/Managers/EnemySpawner.SetShouldPlay` _returnvalue false)
  (bind _outactors (`GameplayStatics.GetAllActorsOfClass` "/Game/Assets/Blueprints/Enemy/True_Cardboard.True_Cardboard_C"))
  (for _array_element _outactors
    (`/Game/Assets/Blueprints/Enemy/True_Cardboard.Reset` _array_element))
  (`/Game/Assets/Blueprints/Player/FirstPersonCharacter.DisablePlayer` (`self.FirstPersonRef`) true)
  (`AudioComponent.Stop` (`self.BGM_Level`))
  (`GameplayStatics.PlaySound2D` "/Game/Assets/Audio/SFX/Environment/SFX_gameOver.SFX_gameOver" 1.0 1.0 0.0 null null)
  (`GameplayStatics.PlaySound2D` "/Game/Assets/Audio/SFX/Environment/SFX_aww_Cue.SFX_aww_Cue" 1.0 1.0 0.0 null null))

(event `StartIntro`
  ;[1 1 1] Start Intro
  (set `PlayerController.bShowMouseCursor` true (`GameplayStatics.GetPlayerController` 0)))

(fn `UserConstructionScript`)