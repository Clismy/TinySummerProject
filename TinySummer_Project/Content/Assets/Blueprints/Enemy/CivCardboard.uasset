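; CivCardboard is a pop-up cardboard target that awards score and time through GameTimer when hit.
; The hit component's name (Head, Body or Feet) selects the reward, and the target plays its despawn animation.
; Activate plays the spawn animation and shortens DeathRate by 5% each time, with no clamp applied.
; Tick retires a live target without reward once DeathTimer reaches DeathRate.
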(event `Hit`
  (params (HitCompontent :type "ActorComponent Object Reference") (GotHit :type Boolean))
  (if (not (`self.IsDead`))
    (set `self.IsDead` true)
    (`/Engine/EditorBlueprintResources/StandardMacros.IsValid` HitCompontent
      (:`Is Valid`
        (switch `string` (`KismetSystemLibrary.GetObjectName` HitCompontent)
          (:`Head`
            (set `self.ScoreToAdd` (`self.HeadScore`))
            (set `self.TimeToAdd` (`self.HeadTime`)))
          (:`Body`
            (set `self.ScoreToAdd` (`self.BodyScore`))
            (set `self.TimeToAdd` (`self.BodyTime`)))
          (:`Feet`
            (set `self.ScoreToAdd` (`self.FeetScore`))
            (set `self.TimeToAdd` (`self.FeetTime`)))))
      (:`Is Not Valid`
        _))
    (`|ExecutionSequence`
      (:`then_0`
        (`SkeletalMeshComponent.PlayAnimation` (`self.SkeletalMesh`) "/Game/Assets/Animations/Enemies/ANIM_enemyPopcorn_despawn.ANIM_enemyPopcorn_despawn" false)
        (set `self.DeathTimer` 0.0)
        (`KismetSystemLibrary.PrintString` (`KismetSystemLibrary.GetDisplayName` HitCompontent))
        (bind _returnvalue (`AnimSequenceBase.GetPlayLength` (select `int` 0 :`0` "/Game/Assets/Animations/Enemies/ANIM_enemyPopcorn_despawn.ANIM_enemyPopcorn_despawn" :`1` null :`2` null :!type "AnimSequenceBase Object Reference")))
        (`KismetSystemLibrary.Delay` _returnvalue))
      (:`then_1`
        (if GotHit
          (bind _returnvalue_2 (`GameplayStatics.GetActorOfClass` "/Game/Assets/Blueprints/Managers/GameTimer.GameTimer_C"))
          (`/Game/Assets/Blueprints/Managers/GameTimer.AddScore` _returnvalue_2 (`self.ScoreToAdd`))
          (`/Game/Assets/Blueprints/Managers/GameTimer.AddSeconds` _returnvalue_2 (`self.TimeToAdd`)))))))

(event `self.ReceiveBeginPlay`
  ;[1 1 1] Event Begin
  (bind _returnvalue (`GameplayStatics.GetActorOfClass` "/Game/Assets/Blueprints/Managers/EnemySpawner.EnemySpawner_C"))
  (set `self.Enemy Spawner` _returnvalue))

(event `Activate`
  ;[1 1 1] Activate Cardboard
  (if (`self.IsDead`)
    (set `self.DeathRate` (* (`self.DeathRate`) 0.95))
    (`SkeletalMeshComponent.PlayAnimation` (`self.SkeletalMesh`) "/Game/Assets/Animations/Enemies/ANIM_enemyPopcorn_spawn.ANIM_enemyPopcorn_spawn" false)
    (bind _returnvalue (`AnimSequenceBase.GetPlayLength` (select `int` 0 :`0` "/Game/Assets/Animations/Enemies/ANIM_enemyPopcorn_spawn.ANIM_enemyPopcorn_spawn" :`1` null :`2` null :!type "AnimSequenceBase Object Reference")))
    (`KismetSystemLibrary.Delay` _returnvalue)
    (set `self.IsDead` false)))

(event `self.ReceiveTick`
  (params (DeltaSeconds :type "Float (single-precision)"))
  ;[1 1 1] Update
  (if (`self.IsDead`)
    _
    (elif (>= (`self.DeathTimer`) (`self.DeathRate`))
      (`self.Hit` null)
      (else
        (set `self.DeathTimer` (+ (`self.DeathTimer`) DeltaSeconds))))))

(fn `UserConstructionScript`)