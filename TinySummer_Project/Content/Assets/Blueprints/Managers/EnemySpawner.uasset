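; Enemy spawner manager that activates random Cardboard and CivCardboard targets already in the level while play is enabled.
; BeginPlay gathers both types into lists; activated boards are removed, and AddNewPoints and AddCivPoints put boards back.
; Tick runs two timers with randomized intervals, triggering cardboard batches or single civilians.
; UpdateSettings ramps difficulty by shortening cardboard intervals toward minimum limits and raising the capped batch size.
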(event `self.ReceiveTick`
  (params (DeltaSeconds :type "Float (single-precision)"))
  ;[1 1 1] new spawning
  (if (`self.ShouldPlay`)
    (`|ExecutionSequence`
      (:`then_0`
        (`self.SpawnCheck` DeltaSeconds
          (:`true`
            (`self.SpawnCardboard`))))
      (:`then_1`
        (`self.CivSpawnCheck` DeltaSeconds
          (:`true`
            (`self.SpawnCivCardboard`)))))))

(event `self.ReceiveBeginPlay`
  ;[1 1 1] Event BeginPlay
  (bind _outactors (`GameplayStatics.GetAllActorsOfClass` "/Game/Assets/Blueprints/Enemy/Cardboard.Cardboard_C"))
  (set `self.cardboardList` _outactors)
  (bind _outactors_2 (`GameplayStatics.GetAllActorsOfClass` "/Game/Assets/Blueprints/Enemy/CivCardboard.CivCardboard_C"))
  (set `self.civCardboardList` _outactors_2)
  (set `self.CivSpawnRate` (`KismetMathLibrary.RandomFloatInRange` (`self.secondsToNextSpawnMin`) (`self.secondsToNextSpawn`))))

(event `AddNewPoints`
  (params (Cardboard :type "/Game/Assets/Blueprints/Enemy/Cardboard Object Reference"))
  ;[1 1 1] AddPoint
  (`KismetArrayLibrary.Array_Add` (`self.cardboardList`) Cardboard))

(event `SetShouldPlay`
  (params (ShouldPlay :type Boolean))
  ;[1 1 1] SetShouldPlay
  (bind _output_get (set `self.ShouldPlay` ShouldPlay))
  (if (== _output_get false)
    (set `self.SpawnTimer` 0.0)
    (set `self.CivSpawnTimer` 0.0)))

(event `AddCivPoints`
  (params (CIvCardboard :type "/Game/Assets/Blueprints/Enemy/CivCardboard Object Reference"))
  ;[1 1 1] AddCivPoint
  (`KismetArrayLibrary.Array_Add` (`self.civCardboardList`) CIvCardboard))

(event `UpdateSettings`
  ;[1 1 1] Update Score settings
  (set `self.secondsToNextSpawnMin` (`KismetMathLibrary.FClamp` (* (`self.secondsToNextSpawnMin`) 0.95) (`self.secondsToNextSpawnMinAmount`) 100.0))
  (set `self.secondsToNextSpawn` (`KismetMathLibrary.FClamp` (* (`self.secondsToNextSpawn`) 0.95) (`self.secondsToNextSpawnMaxAmount`) 100.0))
  (set `self.boardsToSpawnCount` (`KismetMathLibrary.Clamp` (+ (`self.boardsToSpawnCount`) 1) 0 4)))

(fn `SpawnCardboard`
  (for _ (range (+ (`KismetMathLibrary.Clamp` (`KismetMathLibrary.RandomInteger` (`self.boardsToSpawnCount`)) 0 (- (`KismetArrayLibrary.Array_Length` (`self.cardboardList`)) 1)) 1))
    (set `self.RandInt` (`KismetMathLibrary.RandomInteger` (- (`KismetArrayLibrary.Array_Length` (`self.cardboardList`)) 1)))
    (`GameplayStatics.GetAllActorsOfClass` "/Game/Assets/Blueprints/Enemy/Cardboard.Cardboard_C")
    (if (not (<= (`KismetArrayLibrary.Array_Length` (`self.cardboardList`)) 0))
      (`/Game/Assets/Blueprints/Enemy/Cardboard.Activate` (`|GetArrayItem` (`self.cardboardList`) (`self.RandInt`)))
      (`KismetArrayLibrary.Array_Remove` (`self.cardboardList`) (`self.RandInt`))))
  (set `self.SpawnRate` (`KismetMathLibrary.RandomFloatInRange` (`self.secondsToNextSpawnMin`) (`self.secondsToNextSpawn`)))
  (set `self.SpawnTimer` 0.0)
  (return))

(fn `SpawnCivCardboard`
  (set `self.RandCivIndex` (`KismetMathLibrary.RandomInteger` (- (`KismetArrayLibrary.Array_Length` (`self.civCardboardList`)) 1)))
  (`GameplayStatics.GetAllActorsOfClass` "/Game/Assets/Blueprints/Enemy/CivCardboard.CivCardboard_C")
  (if (not (<= (`KismetArrayLibrary.Array_Length` (`self.civCardboardList`)) 0))
    (`/Game/Assets/Blueprints/Enemy/CivCardboard.Activate` (`|GetArrayItem` (`self.civCardboardList`) (`self.RandCivIndex`)))
    (`KismetArrayLibrary.Array_Remove` (`self.civCardboardList`) (`self.RandCivIndex`))
    (set `self.CivSpawnTimer` 0.0)
    (set `self.CivSpawnRate` (`KismetMathLibrary.RandomFloatInRange` (`self.secondsToNextCivSpawnMinAmount`) (`self.secondsToNextCivSpawnMaxAmount`)))
    (return)))

(fn `UserConstructionScript`)