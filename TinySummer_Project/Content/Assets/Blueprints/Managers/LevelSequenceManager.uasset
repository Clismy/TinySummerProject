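; LevelSequenceManager is a Blueprint that plays level sequences, including the level's intro camera cutscene.
; SetIntroCutscene finds the LevelManager, plays the CameraToStart sequence, waits out its length with a Delay, then calls StartIntro on the manager.
; PlaySequence stops the current player at its end and creates a new one to play the given sequence forward or in reverse.
; A skip branch exists but is unconnected.
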(event `SetIntroCutscene`
  (bind _returnvalue (`GameplayStatics.GetActorOfClass` "/Game/Assets/Blueprints/Managers/LevelManager.LevelManager_C"))
  (set `self.LevelManagerRef` _returnvalue)
  (bind (_outactor _returnvalue_2) (`LevelSequencePlayer.CreateLevelSequencePlayer` "/Game/CameraToStart.CameraToStart" (`self.SequenceSettings`)))
  (bind _output_get (set `self.SequencePlayer` _returnvalue_2))
  (set `self.SequenceID` 0)
  (set `self.IsClipPlaying` true)
  (`MovieSceneSequencePlayer.Play` _output_get)
  (bind _timelength (`self.TimeLength`))
  (`KismetSystemLibrary.Delay` _timelength)
  (`/Game/Assets/Blueprints/Managers/LevelManager.StartIntro` (`self.LevelManagerRef`)))

(event `PlaySequence`
  (params (levelSequence :type "LevelSequence Object Reference") (playReverse :type Boolean) (sequenceID :type Integer))
  (`MovieSceneSequencePlayer.GoToEndAndStop` (`self.SequencePlayer`))
  (bind (_outactor _returnvalue) (`LevelSequencePlayer.CreateLevelSequencePlayer` levelSequence (`self.SequenceSettings`)))
  (set `self.SequencePlayer` _returnvalue)
  (set `self.sequenceClip` levelSequence)
  (if playReverse
    (`MovieSceneSequencePlayer.PlayReverse` (`self.SequencePlayer`))
    (else
      (`MovieSceneSequencePlayer.Play` (`self.SequencePlayer`)))))

(event `InputAction|F`
  (params (Key :type "Key Structure")))

(fn `IsPlaying`
  (returns (IsPlaying :type Boolean))
  (return (`MovieSceneSequencePlayer.IsPlaying` (`self.SequencePlayer`))))

(fn `TimeLength`
  (returns (TimeLength :type "Float (double-precision)"))
  (return (`TimeManagementBlueprintLibrary.Conv_QualifiedFrameTimeToSeconds` (`MovieSceneSequencePlayer.GetEndTime` (`self.SequencePlayer`)))))

(fn `UserConstructionScript`)