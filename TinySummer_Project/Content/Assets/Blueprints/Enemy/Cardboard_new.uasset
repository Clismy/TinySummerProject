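; Short-lived cardboard target enemy that awards score and extra time when hit.
; The Hit event returns the target's spawn point to its EnemySpawner and destroys the actor, then updates the GameTimer only if it was actually hit.
; An unhit target expires through the same event after a BeginPlay delay, without reward.
; Setter events supply the spawner and spawn point references.
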(event `Hit`
  (params (HitCompontent :type "ActorComponent Object Reference") (GotHit :type Boolean))
  (`|ExecutionSequence`
    (:`then_0`
      (`/Game/Assets/Blueprints/Managers/EnemySpawner.AddPoint` (`self.EnemySpawner`) (`self.SpawnPoint`))
      (`KismetSystemLibrary.PrintString` (`KismetSystemLibrary.GetDisplayName` HitCompontent))
      (`self.K2_DestroyActor`))
    (:`then_1`
      (if GotHit
        (bind _returnvalue (`GameplayStatics.GetActorOfClass` "/Game/Assets/Blueprints/Managers/GameTimer.GameTimer_C"))
        (`/Game/Assets/Blueprints/Managers/GameTimer.AddScore` _returnvalue 20)
        (`/Game/Assets/Blueprints/Managers/GameTimer.AddSeconds` _returnvalue 2)))))

(event `self.ReceiveBeginPlay`
  (`KismetSystemLibrary.Delay` 10.0)
  (`self.Hit` null))

(event `SetEnemySpawner`
  (params (EnemySpawner :type "/Game/Assets/Blueprints/Managers/EnemySpawner Object Reference"))
  (set `self.EnemySpawner` EnemySpawner))

(event `SetSpawnPoint`
  (params (SpawnPoint :type "/Game/Assets/Blueprints/Enemy/SpawnPoint Object Reference"))
  (set `self.SpawnPoint` SpawnPoint))

(fn `UserConstructionScript`)