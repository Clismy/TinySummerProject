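; Level manager Blueprint that switches the game between the 3D menu and first-person play through two events.
; SwitchToMenu disables player input, shows the cursor, halts the EnemySpawner and moves the view target to BP_Menu3D.
; SwitchToPlayer targets the character's CameraPos, then after a delay restores input, starts GameTimer and spawning, and creates the HUD.
; Both create Level Sequence players for camera transitions; older camera and menu-widget nodes remain unconnected.
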(event `self.ReceiveBeginPlay`)

(event `SwitchToMenu`
  ;[1 1 1] Switch To Menu
  (bind _returnvalue (`GameplayStatics.GetActorOfClass` "/Game/Assets/Blueprints/Menus/BP_Menu3D.BP_Menu3D_C"))
  (`self.DisableInput` (`GameplayStatics.GetPlayerCharacter` 0) (`GameplayStatics.GetPlayerController` 0))
  (set `PlayerController.bShowMouseCursor` true (`GameplayStatics.GetPlayerController` 0))
  (bind _returnvalue_2 (`GameplayStatics.GetActorOfClass` "/Game/Assets/Blueprints/Managers/EnemySpawner.EnemySpawner_C"))
  (`/Game/Assets/Blueprints/Managers/EnemySpawner.SetShouldPlay` _returnvalue_2 false)
  (bind _returnvalue_3 (`GameplayStatics.GetActorOfClass` "/Game/Assets/Blueprints/Menus/BP_Menu3D.BP_Menu3D_C"))
  (`PlayerController.SetViewTargetWithBlend` (`GameplayStatics.GetPlayerController` 0) _returnvalue_3 0.0 "VTBlend_Linear" 0.0 false)
  (`LevelSequencePlayer.CreateLevelSequencePlayer` "/Game/CameraToMenu.CameraToMenu" (`self.Settings`)))

(event `SwitchToPlayer`
  ;[1 1 1] Switch To Player
  (bind _asfirst_person_character (cast `/Game/Assets/Blueprints/Player/FirstPersonCharacter` (`GameplayStatics.GetPlayerCharacter` 0)))
  (`PlayerController.SetViewTargetWithBlend` (`GameplayStatics.GetPlayerController` 0) (`/Game/Assets/Blueprints/Player/FirstPersonCharacter.CameraPos` _asfirst_person_character) 0.0 "VTBlend_Linear" 0.0 false)
  (`LevelSequencePlayer.CreateLevelSequencePlayer` "/Game/CameraToPlayer.CameraToPlayer" (`self.Settings_Player`))
  (`KismetSystemLibrary.Delay` 2.0)
  (`self.EnableInput` (`GameplayStatics.GetPlayerCharacter` 0) (`GameplayStatics.GetPlayerController` 0))
  (set `PlayerController.bShowMouseCursor` false (`GameplayStatics.GetPlayerController` 0))
  (bind _returnvalue (`GameplayStatics.GetActorOfClass` "/Game/Assets/Blueprints/Managers/GameTimer.GameTimer_C"))
  (`/Game/Assets/Blueprints/Managers/GameTimer.SetPlayTimer` _returnvalue true)
  (bind _returnvalue_2 (`GameplayStatics.GetActorOfClass` "/Game/Assets/Blueprints/Managers/EnemySpawner.EnemySpawner_C"))
  (`/Game/Assets/Blueprints/Managers/EnemySpawner.SetShouldPlay` _returnvalue_2 true)
  (bind _returnvalue_3 (`|CreateWidget` "/Game/Assets/Widgets/WBP_HUD.WBP_HUD_C" (`GameplayStatics.GetPlayerController` 0)))
  (`UserWidget.AddToViewport` _returnvalue_3 0))

(fn `UserConstructionScript`)